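; Capturer actor that photographs its parent actor and extra actors from many angles, then uploads via BP_CaptureUploader, relaying QR and checkout results.
; Construction builds a spherical spiral spline of inward-facing camera points, supplemented by BP_ExtraCapture transforms.
; Three scene captures feed materials that export masked PNGs and optional depth maps, looped instantly or with delay.
; Camera intrinsics and converted per-frame matrices go to transforms.json; Android skips mask compositing.
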(event Custom|Capture
  (params (bAsync :type Boolean))
  (bind _framecount (Variables|CaptureParameters|GetFrameCount))
  (bind _extraframes (Variables|Default|GetExtraFrames))
  (bind _extraframes_2 (Variables|Default|GetExtraFrames))
  (bind _returnvalue (Utilities|Array|Length _extraframes_2))
  (bind _returnvalue_2 (- _framecount 1))
  (bind _returnvalue_3 (- _returnvalue 1))
  (Class|IGCFunctionLibrary|DeleteAllCaptures (Utilities|String|Append (Variables|Others|GetCapturePath) "/images/"))
  (CallFunction|SetShowOnlyActors)
  (Development|PrintString "Capture Starting" true true "(R=0.122139,G=0.043735,B=0.791298,A=1.000000)" 5.0)
  (Variables|Default|SetCurrentStage "NewEnumerator1")
  (CallFunction|SetRenderingSettings)
  (if bAsync
    (bind _index (Utilities|ForLoopwithDelay 0 _returnvalue_2 0.0)
      (:Body
        (CallFunction|ExportSingleCapture :index _index))
      (:Completed
        (bind _index_2 (Utilities|ForLoopwithDelay 0 _returnvalue_3 0.0)
          (:Body
            (CallFunction|ExportSingleCapture (+ (Variables|CaptureParameters|GetFrameCount) _index_2) (Transformation|GetActorTransform (Utilities|Array|Get(acopy) _extraframes _index_2)) true))
          (:Completed
            (CallFunction|FinishCapture :!label _label)
            (Variables|Default|SetCurrentStage "NewEnumerator0")
            (Default|CallOnCaptureFinished)))))
    (else
      (for _index_3 (range 0 _returnvalue_2)
        (CallFunction|ExportSingleCapture :index _index_3))
      (for _index_4 (range 0 _returnvalue_3)
        (CallFunction|ExportSingleCapture (+ _index_4 (Variables|CaptureParameters|GetFrameCount)) (Transformation|GetActorTransform (Utilities|Array|Get(acopy) _extraframes _index_4)) true))
      (goto _label))))

(event Custom|UploadCaptures
  (Utilities|IsValid (Variables|Others|GetCaptureUploader)
    (:Is%20Valid
      (Development|PrintString "Already Uploading to API" true true "(R=0.122139,G=0.043735,B=0.791298,A=1.000000)" 5.0))
    (:Is%20Not%20Valid
      (bind _returnvalue (Game|SpawnActorfromClass "/IGC_UE/Blueprints/BP_CaptureUploader.BP_CaptureUploader_C" (Math|Transform|MakeTransform "0, 0, 0") "Undefined" "OverrideRootScale" 0 (Variables|CaptureParameters|GetAPI_Key) 0.0 0))
      (bind _output_get (Variables|Others|SetCaptureUploader _returnvalue))
      (Variables|Default|SetCurrentStage "NewEnumerator2")
      (EventDispatchers|BindEventtoOnQRReceived _output_get (EventDispatchers|CreateEvent :!event Finish))
      (EventDispatchers|BindEventtoOnCheckout _output_get (EventDispatchers|CreateEvent :!event CheckoutStart)))))

(event Custom|CaptureAndUpload
  (params (bAsyncCapture :type Boolean))
  (EventDispatchers|BindEventtoOnCaptureFinished (EventDispatchers|CreateEvent :!event Custom|UploadCaptures))
  (CallFunction|Capture bAsyncCapture))

(event EventBeginPlay
  (CallFunction|SetUpRenderTargets)
  (Variables|Others|SetCapturePath (CallFunction|GetCapturePath))
  (bind _outactors (Actor|GetAllActorsOfClass "/IGC_UE/Blueprints/BP_ExtraCapture.BP_ExtraCapture_C"))
  (Variables|Default|SetExtraFrames _outactors))

(event Input|KeyboardEvents|L
  (params (Key :type Key%20Structure :default "None"))
  ;[0.5457 1 0.6105] Use Example
)

(event Input|KeyboardEvents|J
  (params (Key :type Key%20Structure :default "None"))
  ;[0.5457 1 0.6105] Use Example
)

(event Input|KeyboardEvents|K
  (params (Key :type Key%20Structure :default "None"))
  ;[0.5457 1 0.6105] Use Example
)

(fn ConstructionScript
  (bind _framecount (Variables|CaptureParameters|GetFrameCount))
  (bind _zenithclamp (Variables|CaptureParameters|GetZenithClamp))
  (bind _camerapath (Variables|Default|GetCameraPath))
  (bind _output_get (Variables|/Script/Engine.SceneCaptureComponent2D|SetFOVAngle (Variables|Default|GetSceneCaptureComponent2D_Mask) (Variables|CaptureParameters|GetCameraFOV)))
  (bind _output_get_2 (Variables|/Script/Engine.SceneCaptureComponent2D|SetFOVAngle (Variables|Default|GetSceneCaptureComponent2D) _output_get))
  (Variables|/Script/Engine.SceneCaptureComponent2D|SetFOVAngle (Variables|Default|GetSceneCaptureComponent2D_Depth) _output_get_2)
  (bind _coordinate (CallFunction|GetSphericalCoordinates 0.0 0.0 (Variables|CaptureParameters|GetRadius)))
  (Spline|ClearSplinePoints _camerapath true)
  (Transformation|SetRelativeLocation _camerapath _coordinate false true)
  (for _index (range 0 (- _framecount 1))
    (bind _coordinate_2 (CallFunction|GetSphericalCoordinates (* (Variables|CaptureParameters|GetPathXSpeed) 3.141593 2.0 (/ (Math|Conversions|ToFloat(Integer) _index) (Math|Conversions|ToFloat(Integer) _framecount))) (* (Math|Float|MapRangeClamped (/ (Math|Conversions|ToFloat(Integer) _index) (Math|Conversions|ToFloat(Integer) _framecount)) 0.0 1.0 (.x _zenithclamp) (.y _zenithclamp)) 3.141593) (Variables|CaptureParameters|GetRadius)))
    (Spline|AddSplinePoint (Variables|Default|GetCameraPath) _coordinate_2 "Local" true))
  (CallFunction|SetCameraTransformatPoint :PointIndex (Variables|Others|GetStartingPointIndex)))

(fn GetSphericalCoordinates
  (params (theta :type Float%20%28double-precision%29) (phi :type Float%20%28double-precision%29) (radius :type Float%20%28double-precision%29))
  (return (Math|Vector|MakeVector (|((r*(sin(phi)))*(cos(theta))) theta phi radius) (|((r*(sin(phi)))*(sin(theta))) theta phi radius) (- (|(r*(cos(phi))) phi radius) (/ (Variables|CaptureParameters|GetRadius) 2.0)))))

(fn SetCameraTransformatPoint
  (params (PointIndex :type Integer) (Transform :type Transform) (bIsExtraFrame :type Boolean))
  (bind _location (Math|Transform|BreakTransform Transform))
  (bind _scenecapturecomponent2d (Variables|Default|GetSceneCaptureComponent2D))
  (bind _camerapath (Variables|Default|GetCameraPath))
  (bind _returnvalue (Spline|GetLocationatSplinePoint _camerapath PointIndex "World"))
  (bind _returnvalue_2 (select bIsExtraFrame _location _returnvalue))
  (Transformation|SetWorldLocation _scenecapturecomponent2d _returnvalue_2 false true)
  (Transformation|SetWorldRotation _scenecapturecomponent2d (select bIsExtraFrame (.Rotation (Math|Transform|BreakTransform Transform)) (Math|Rotator|FindLookatRotation _returnvalue_2 (Transformation|GetActorLocation))) false false))

(fn GetCameraLTransform
  (bind _returnvalue (Game|GetPlatformName))
  (bind _returnvalue_2 (Math|Transform|MakeTransform "0, 0, 0" "0.000000,270.000000,270.000000"))
  (bind _scenecapturecomponent2d (Variables|Default|GetSceneCaptureComponent2D))
  (bind _returnvalue_3 (Utilities|Enum|Equal(Enum) _returnvalue "Android"))
  (bind _returnvalue_4 (Transformation|GetRelativeTransform _scenecapturecomponent2d))
  (bind (_location _rotation _scale) (Math|Transform|BreakTransform _returnvalue_4))
  (bind _returnvalue_5 (Math|Rotator|Delta(Rotator) _rotation "0, 0,-180.000000"))
  (bind _returnvalue_6 (Math|Transform|MakeTransform _location _returnvalue_5 _scale))
  (bind _returnvalue_7 (Math|Transform|SelectTransform _returnvalue_6 _returnvalue_4 _returnvalue_3))
  (bind _returnvalue_8 (Math|Transform|ComposeTransforms _returnvalue_2 _returnvalue_7))
  (bind (_location_2 _rotation_2 _scale_2) (Math|Transform|BreakTransform _returnvalue_8))
  (bind (_roll _pitch _yaw) (Math|Rotator|BreakRotator _rotation_2))
  (return (Math|Transform|ToMatrix(Transform) (Math|Transform|MakeTransform (* (* (/ _location_2 1e+02) "-1.000000,1.000000,1.000000") (Variables|CaptureParameters|GetScaleMult)) (Math|Rotator|MakeRotator _roll (* _pitch -1.0) (* _yaw -1.0)) _scale_2))))

(fn SetShowOnlyActors
  (bind _returnvalue (Actor|GetAttachParentActor))
  (bind _actors (LocalVariables|GetActors))
  (Utilities|Array|Add _actors _returnvalue)
  (Utilities|Array|AppendArray _actors (Actor|GetAttachedActors _returnvalue true false))
  (for _array_element (Variables|CaptureParameters|GetExtraActors)
    (if (> (Utilities|Array|Length (Actor|GetAttachedActors _array_element true false)) 0)
      (Utilities|Array|AppendArray (LocalVariables|GetActors) (Actor|GetAttachedActors _array_element true false))))
  (Utilities|Array|AppendArray (LocalVariables|GetActors) (Variables|CaptureParameters|GetExtraActors))
  (bind _output_get (Variables|/Script/Engine.SceneCaptureComponent|SetShowOnlyActors (Variables|Default|GetSceneCaptureComponent2D) (LocalVariables|GetActors)))
  (bind _output_get_2 (Variables|/Script/Engine.SceneCaptureComponent|SetShowOnlyActors (Variables|Default|GetSceneCaptureComponent2D_Mask) _output_get))
  (Variables|/Script/Engine.SceneCaptureComponent|SetShowOnlyActors (Variables|Default|GetSceneCaptureComponent2D_Depth) _output_get_2))

(fn ExportSingleCapture
  (params (index :type Integer) (Transform :type Transform) (bIsExtraFrame :type Boolean))
  (bind _returnvalue (Utilities|String|ToString(Integer) index))
  (bind _depthmaterial (Variables|Others|GetDepthMaterial))
  (bind _scenecapturecomponent2d_mask (Variables|Default|GetSceneCaptureComponent2D_Mask))
  (bind _capturematerial (Variables|Others|GetCaptureMaterial))
  (bind _scenecapturecomponent2d (Variables|Default|GetSceneCaptureComponent2D))
  (bind _exportrendertarget (Variables|Others|GetExportRenderTarget))
  (bind _exportrendertarget_2 (Variables|Others|GetExportRenderTarget))
  (bind _scenecapturecomponent2d_depth (Variables|Default|GetSceneCaptureComponent2D_Depth))
  (Utilities|FlowControl|Sequence
    (:then_0
      (LocalVariables|Setfilename (Utilities|String|Append "" (Utilities|Select :Index (Utilities|String|Len _returnvalue) :Option%200 "000" :Option%201 "00" :Option%202 "0") _returnvalue ".png"))
      (LocalVariables|Setfilepath (Utilities|String|Append (Variables|Others|GetCapturePath) "/images")))
    (:then_1
      (CallFunction|SetCameraTransformatPoint index Transform bIsExtraFrame)
      (Rendering|SceneCapture|CaptureScene _scenecapturecomponent2d :!class /Script/Engine.SceneCaptureComponent2D)
      (if (Utilities|Enum|Equal(Enum) (Game|GetPlatformName) "Android")
        (Rendering|ExportRenderTarget (Variables|/Script/Engine.SceneCaptureComponent2D|GetTextureTarget _scenecapturecomponent2d) (LocalVariables|Getfilepath) (LocalVariables|Getfilename))
        (else
          (Rendering|SceneCapture|CaptureScene _scenecapturecomponent2d_mask :!class /Script/Engine.SceneCaptureComponent2D)
          (Rendering|Material|SetTextureParameterValue (Variables|Others|GetCaptureMaterial) "MaskTexture" (Variables|/Script/Engine.SceneCaptureComponent2D|GetTextureTarget _scenecapturecomponent2d_mask))
          (Rendering|Material|SetTextureParameterValue _capturematerial "Texture" (Variables|/Script/Engine.SceneCaptureComponent2D|GetTextureTarget (Variables|Default|GetSceneCaptureComponent2D)))
          (Rendering|DrawMaterialtoRenderTarget _exportrendertarget _capturematerial)
          (Rendering|ExportRenderTarget _exportrendertarget (LocalVariables|Getfilepath) (LocalVariables|Getfilename)))))
    (:then_2
      (if (Variables|Default|GetbExportDepthMaps)
        (Rendering|SceneCapture|CaptureScene _scenecapturecomponent2d_depth :!class /Script/Engine.SceneCaptureComponent2D)
        (Rendering|Material|SetTextureParameterValue _depthmaterial "Texture" (Variables|/Script/Engine.SceneCaptureComponent2D|GetTextureTarget _scenecapturecomponent2d_depth))
        (Rendering|DrawMaterialtoRenderTarget _exportrendertarget_2 _depthmaterial)
        (Rendering|ExportRenderTarget _exportrendertarget_2 (LocalVariables|Getfilepath) (Utilities|String|Append "d_" (LocalVariables|Getfilename)))
        (Rendering|ClearRenderTarget2D (Variables|Others|GetDepthRenderTarget) "(R=0.000000,G=0.000000,B=0.000000,A=0.000000)")))
    (:then_3
      (Utilities|Array|Add (Variables|Others|GetFrames) (Utilities|Struct|MakeFrameInformation (Utilities|String|Append "./images/" (LocalVariables|Getfilename)) 5e+01 (CallFunction|GetCameraLTransform)))
      (Rendering|ClearRenderTarget2D (Variables|Others|GetRenderTarget))
      (Rendering|ClearRenderTarget2D (Variables|Others|GetMaskRenderTarget) "(R=0.000000,G=0.000000,B=0.000000,A=0.000000)")
      (Rendering|ClearRenderTarget2D (Variables|Others|GetExportRenderTarget) "(R=0.000000,G=0.000000,B=0.000000,A=0.000000)"))))

(fn FinishCapture
  (bind _focallength (CallFunction|GetFocalLength))
  (bind _scenecapturecomponent2d (Variables|Default|GetSceneCaptureComponent2D))
  (bind _rendersize (Variables|CaptureParameters|GetRenderSize))
  (bind _returnvalue (Math|Conversions|ToFloat(Integer) _rendersize))
  (bind _fovangle (Variables|/Script/Engine.SceneCaptureComponent2D|GetFOVAngle _scenecapturecomponent2d))
  (bind _returnvalue_2 (Math|Trig|DegreesToRadians _fovangle))
  (bind _returnvalue_3 (/ _returnvalue 2.0))
  (Development|PrintString "Capturing Finished" true true "(R=0.122139,G=0.043735,B=0.791298,A=1.000000)" 5.0)
  (Class|IGCFunctionLibrary|SaveCaptureInformationtoJSON (Utilities|String|Append (Class|KismetSystemLibrary|GetProjectDirectory) "/OUTPUTS/Capture/transforms.json") (Utilities|Struct|MakeCaptureInformation _returnvalue_2 _returnvalue_2 _focallength _focallength 0.0 0.0 0.0 0.0 _returnvalue_3 _returnvalue_3 _returnvalue _returnvalue 64 (Variables|Others|GetFrames)))
  (Rendering|ClearRenderTarget2D (Variables|Others|GetRenderTarget))
  (Rendering|ClearRenderTarget2D (Variables|Others|GetExportRenderTarget) "(R=0.000000,G=0.000000,B=0.000000,A=0.000000)")
  (Rendering|ClearRenderTarget2D (Variables|Others|GetMaskRenderTarget))
  (Utilities|Array|Clear (Variables|Others|GetFrames)))

(fn Finish
  (params (bSucceeded :type Boolean) (Message :type String) (QRTexture :type Texture%202D%20Object%20Reference) (CheckoutURL :type String))
  (Variables|Default|SetCurrentStage "NewEnumerator0")
  (Default|CallOnUploadFinished bSucceeded Message QRTexture CheckoutURL))

(fn CheckoutStart
  (Variables|Default|SetCurrentStage "NewEnumerator3"))

(fn SetUpRenderTargets
  (bind _rendersize (Variables|CaptureParameters|GetRenderSize))
  (bind _rendersize_2 (Variables|CaptureParameters|GetRenderSize))
  (bind _rendersize_3 (Variables|CaptureParameters|GetRenderSize))
  (bind _rendersize_4 (Variables|CaptureParameters|GetRenderSize))
  (bind _returnvalue (* _rendersize 2))
  (Utilities|FlowControl|Sequence
    (:then_0
      (bind _returnvalue_2 (Rendering|CreateRenderTarget2D _returnvalue _returnvalue "RTF_RGBA8_SRGB"))
      (bind _output_get (Variables|Others|SetRenderTarget _returnvalue_2))
      (Variables|/Script/Engine.SceneCaptureComponent2D|SetTextureTarget (Variables|Default|GetSceneCaptureComponent2D) _output_get)
      (bind _returnvalue_3 (Rendering|Material|CreateDynamicMaterialInstance "/IGC_UE/Materials/M_CaptureEditor.M_CaptureEditor" "None" "Transient" :!class /Script/Engine.KismetMaterialLibrary))
      (Variables|Others|SetCaptureMaterial _returnvalue_3)
      (bind _returnvalue_4 (Rendering|CreateRenderTarget2D _rendersize_2 _rendersize_2 "RTF_RGBA8_SRGB" "(R=0.000000,G=0.000000,B=0.000000,A=0.000000)"))
      (Variables|Others|SetExportRenderTarget _returnvalue_4)
      (bind _returnvalue_5 (Rendering|CreateRenderTarget2D _rendersize_4 _rendersize_4 "RTF_RGBA8_SRGB" "(R=0.000000,G=0.000000,B=0.000000,A=0.000000)"))
      (bind _output_get_2 (Variables|Others|SetMaskRenderTarget _returnvalue_5))
      (Variables|/Script/Engine.SceneCaptureComponent2D|SetTextureTarget (Variables|Default|GetSceneCaptureComponent2D_Mask) _output_get_2))
    (:then_1
      (if (Variables|Default|GetbExportDepthMaps)
        (bind _returnvalue_6 (Rendering|CreateRenderTarget2D _rendersize_3 _rendersize_3 "RTF_RGBA32f"))
        (bind _output_get_3 (Variables|Others|SetDepthRenderTarget _returnvalue_6))
        (Variables|/Script/Engine.SceneCaptureComponent2D|SetTextureTarget (Variables|Default|GetSceneCaptureComponent2D_Depth) _output_get_3)
        (bind _returnvalue_7 (Rendering|Material|CreateDynamicMaterialInstance "/IGC_UE/Materials/M_DepthEditor.M_DepthEditor" "None" "Transient" :!class /Script/Engine.KismetMaterialLibrary))
        (bind _output_get_4 (Variables|Others|SetDepthMaterial _returnvalue_7))
        (Rendering|Material|SetScalarParameterValue _output_get_4 "MaxDistance" (* (Variables|CaptureParameters|GetRadius) 2.0) :!class /Script/Engine.MaterialInstanceDynamic)))))

(fn SetRenderingSettings
  (bind _capturematerial (Variables|Others|GetCaptureMaterial))
  (Rendering|Material|SetScalarParameterValue _capturematerial "Brightness" (Variables|RenderParameters|GetBrightness) :!class /Script/Engine.MaterialInstanceDynamic)
  (Rendering|Material|SetScalarParameterValue _capturematerial "Contrast" (Variables|RenderParameters|GetContrast) :!class /Script/Engine.MaterialInstanceDynamic)
  (Rendering|Material|SetScalarParameterValue _capturematerial "Desaturation" (Variables|RenderParameters|GetDesaturation) :!class /Script/Engine.MaterialInstanceDynamic)
  (Rendering|Material|SetScalarParameterValue (Variables|Others|GetCaptureMaterial) "Gamma" (Math|Float|SelectFloat 4.0 1.0 (Utilities|Enum|Equal(Enum) (Game|GetPlatformName) "Android")) :!class /Script/Engine.MaterialInstanceDynamic)
  (if (Utilities|Enum|Equal(Enum) (Game|GetPlatformName) "Android")
    (Variables|/Script/Engine.SceneCaptureComponent|SetCaptureSource (Variables|Default|GetSceneCaptureComponent2D) "SCS_SceneColorHDR"))
  (if (not (Variables|RenderParameters|GetbCustomizeShowFlags))
    (Variables|/Script/Engine.SceneCaptureComponent|SetbAlwaysPersistRenderingState (Variables|Default|GetSceneCaptureComponent2D) (Variables|RenderParameters|GetbIsUsingPostProcessing))))

(fn GetFocalLength
  (return (|(x/(2*(tan((FOV/2))))) (Math|Conversions|ToFloat(Integer) (Variables|CaptureParameters|GetRenderSize)) (Math|Trig|DegreesToRadians (Variables|/Script/Engine.SceneCaptureComponent2D|GetFOVAngle (Variables|Default|GetSceneCaptureComponent2D))))))

(fn GetCapturePath
  (return (Utilities|String|SelectString (Class|IGCFunctionLibrary|GetAndroidCapturePath) (Utilities|String|Append (Class|KismetSystemLibrary|GetProjectDirectory) "/OUTPUTS/Capture") (Utilities|Enum|Equal(Enum) (Game|GetPlatformName) "Android"))))