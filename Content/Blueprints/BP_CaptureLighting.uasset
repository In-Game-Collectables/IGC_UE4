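; BP_CaptureLighting is a rig of four point lights sized by a single Radius value, with a Preview component that is destroyed on BeginPlay.
; The construction script passes each light to SetLightRadius, which scales its relative location by Radius against a baseline of 100.
; The same function sets intensity and attenuation radius in linear proportion to Radius, so layout, brightness and reach change together.
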(event EventBeginPlay
  (Components|DestroyComponent (Variables|Default|GetPreview)))

(event Collision|EventActorBeginOverlap
  (params (OtherActor :type Actor%20Object%20Reference)))

(event EventTick
  (params (DeltaSeconds :type Float%20%28single-precision%29)))

(fn ConstructionScript
  (for _array_element (Utilities|Array|MakeArray (Variables|Default|GetPointLight1) (Variables|Default|GetPointLight2) (Variables|Default|GetPointLight3) (Variables|Default|GetPointLight))
    (CallFunction|SetLightRadius _array_element)))

(fn SetLightRadius
  (params (Light :type Point%20Light%20Component%20Object%20Reference))
  (Transformation|SetRelativeLocation Light (* (Variables|/Script/Engine.SceneComponent|GetRelativeLocation Light) (/ (Variables|Default|GetRadius) 1e+02)) false true)
  (Rendering|Components|Light|SetIntensity Light (* 50 (Variables|Default|GetRadius)))
  (Rendering|Lighting|SetAttenuationRadius Light (* 2 (Variables|Default|GetRadius))))