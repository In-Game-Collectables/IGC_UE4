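; Short-lived actor that uploads the project's capture output folder to an external API and retrieves a checkout QR code.
; BeginPlay validates the API key and starts the upload with optional scale and a platform note.
; A successful upload triggers checkout, whose callback broadcasts the QR texture, URL and message through OnQRCodeReceived.
; Failures broadcast through the same dispatcher, and the actor destroys itself when finished.
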(event Custom|UploadComplete
  (params (bSucceeded :type Boolean) (Message :type String) (CheckoutURL :type String))
  (Development|PrintString Message true true "(R=0.122139,G=0.043735,B=0.791298,A=1.000000)" 1e+01)
  (if bSucceeded
    (EventDispatchers|BindEventtoOnQRReceived (delegate Custom|QRCodeReceived))
    ;[1 1 1] Gets QR Code from API.
    ; Calls QRCodeReceived when done.
    (Class|CaptureUploader|Checkout (Variables|Default|GetCaptureFolder) CheckoutURL)
    (Default|CallOnCheckout)
    (else
      (Default|CallOnQRCodeReceived false 0 CheckoutURL Message)
      (CallFunction|Finish))))

(event Custom|QRCodeReceived
  (params (bSucceeded :type Boolean) (Message :type String) (QRTexture :type Texture%202D%20Object%20Reference) (CheckoutURL :type String))
  (Development|PrintString Message true true "(R=0.122139,G=0.043735,B=0.791298,A=1.000000)")
  (Default|CallOnQRCodeReceived bSucceeded QRTexture CheckoutURL Message)
  (CallFunction|Finish))

(event Custom|Finish
  (Actor|DestroyActor))

(event EventBeginPlay
  (bind _returnvalue (Utilities|String|MakeLiteralString "Error: API_Key is empty."))
  (bind _apiscale (Variables|Default|GetAPIScale))
  (if (Utilities|Enum|NotEqual(Enum) (Variables|Default|GetAPIKey) "")
    (Development|PrintString "Upload Starting" true true "(R=0.122139,G=0.043735,B=0.791298,A=1.000000)" 5.0)
    (EventDispatchers|AssignOnUploadCompleted (delegate Custom|UploadComplete))
    (bind _output_get (Variables|Default|SetCaptureFolder (Utilities|String|Append (Class|KismetSystemLibrary|GetProjectDirectory) "/OUTPUTS/Capture")))
    (Class|CaptureUploader|UploadCaptures _output_get (Variables|Default|GetAPIKey) (Utilities|String|SelectString "" (Utilities|String|ToString(Float) _apiscale) (<= _apiscale 0.0)) (CallFunction|GetAPINotes))
    (else
      (Development|PrintString _returnvalue true true "(R=0.122139,G=0.043735,B=0.791298,A=1.000000)" 1e+01)
      (Default|CallOnQRCodeReceived false 0 "" _returnvalue)
      (CallFunction|Finish))))

(fn ConstructionScript)

(fn GetAPINotes
  (return (Utilities|String|Append "Platform: " (Game|GetPlatformName))))